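; BP_Fence is a construction-time actor that places fence poles along an editable spline.
; The Construction Script calls RedrawFence, which assigns the chosen mesh to an Instanced Static Mesh and clears old instances.
; It then divides the spline length by the post spacing and adds instances at even distances in local space.
; All poles share one rotation and scale rather than following the spline's direction.
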(fn `Redraw Fence`
  (bind _instancedstaticmesh (`self.InstancedStaticMesh`))
  (`|ExecutionSequence`
    (:`then_0`
      ;[1 1 1] Setup Mesh and Clear all instances
      (`StaticMeshComponent.SetStaticMesh` _instancedstaticmesh (`self.Mesh`))
      (`InstancedStaticMeshComponent.ClearInstances` _instancedstaticmesh))
    (:`then_1`
      ;[1 1 1] Add all Pole instances
      (bind _spline_distance (`self.Spline Distance`))
      (bind _output_get (set `self.Poles` (`KismetMathLibrary.FFloor` (/ _spline_distance (`self.Posts distance`)))))
      (for _index (range _output_get)
        (`InstancedStaticMeshComponent.AddInstance` (`self.InstancedStaticMesh`) (`KismetMathLibrary.MakeTransform` (`SplineComponent.GetLocationAtDistanceAlongSpline` (`self.Spline`) (* _index (`self.Posts distance`)) "Local") (`self.Poles Rotation`) (`self.Poles Scale`)) false)))))

(fn `Spline Distance`
  (returns (`Spline Distance` :type "Float (single-precision)"))
  (return (`SplineComponent.GetDistanceAlongSplineAtSplinePoint` (`self.Spline`) (- (`SplineComponent.GetNumberOfSplinePoints` (`self.Spline`)) 1))))

(fn `UserConstructionScript`
  (`self.Redraw Fence`))