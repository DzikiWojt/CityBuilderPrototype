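; Base agent actor that can be assigned to buildings and shows a name widget when hovered or selected.
; On assignment it stops the previous building's interactions, walks to the new one via AI MoveTo and, on arrival, runs each of that building's interactions with itself as the agent.
; It spawns its default controller on BeginPlay and, while the name widget is visible, turns it each tick toward the BP_StaticPawn camera.
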(event `self.ReceiveTick`
  (params (DeltaSeconds :type "Float (single-precision)"))
  (if (`self.Is Widget Visible`)
    (`self.Face Widget Name to Camera`)))

(event `self.ReceiveBeginPlay`
  (`self.SpawnDefaultController`))

(event `Assign to Building`
  (params (Building :type "/Game/TitanGamez/Buildings/BP_Building_Base Object Reference"))
  ;[1 1 1] Assign to Building
  (`|ExecutionSequence`
    (:`then_0`
      (`/Engine/EditorBlueprintResources/StandardMacros.IsValid` (`self.Building Assigned`) ; Be sure this is not the first time we assign\nbuilding - if yes, ignore stopping current\ninteractions
        (:`Is Valid`
          (`self.Stop Interactions`))))
    (:`then_1`
      (bind _output_get (set `self.Building Assigned` Building))
      (`|AIMoveTo` self (0.0 0.0 0.0) _output_get 15.0 true
        (:`OnSuccess`
          (`self.Do Interactions`))))))

(event `Do Interactions`
  ;[1 1 1] Do Interactions
  (for _array_element (`Building_Base.Interactions` (`self.Building Assigned`))
    (`Interaction_Base.DoInteraction` _array_element (`self.Building Assigned`) self)))

(event `Stop Interactions`
  ;[1 1 1] Stop Interactions
  (for _array_element (`Building_Base.Interactions` (`self.Building Assigned`))
    (`Interaction_Base.StopInteraction` _array_element (`self.Building Assigned`) self)))

(event `Face Widget Name to Camera`
  ;[1 1 1] Face Widget Name to Camera
  (bind _asbp_static_pawn (cast `/Game/TitanGamez/Game/BP_StaticPawn` (`GameplayStatics.GetPlayerPawn` 0)))
  (`SceneComponent.K2_SetWorldRotation` (`self.WidgetName`) (`KismetMathLibrary.FindLookAtRotation` (`SceneComponent.K2_GetComponentLocation` (`self.WidgetName`)) (`SceneComponent.K2_GetComponentLocation` (`/Game/TitanGamez/Game/BP_StaticPawn.Camera` _asbp_static_pawn))) false false))

(event `Setup Widget`
  (params (`Is Hover ?` :type Boolean) (`Is Selected ?` :type Boolean))
  ;[1 1 1] Setup Widget
  (bind _output_get (set `self.Is Widget Visible` (or `Is Hover ?` `Is Selected ?`)))
  (if _output_get
    (`SceneComponent.SetVisibility` (`self.WidgetName`) true false)
    (bind _asumg_agent_name (cast `/Game/TitanGamez/UI/UMG_AgentName` (`WidgetComponent.GetUserWidgetObject` (`self.WidgetName`))))
    (`/Game/TitanGamez/UI/UMG_AgentName.Setup` _asumg_agent_name (`self.Name`) `Is Hover ?` `Is Selected ?`)
    (else
      (`SceneComponent.SetVisibility` (`self.WidgetName`) false false))))

(fn `UserConstructionScript`)