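; BP_Agent is an AI-driven agent that can be assigned to a building and runs that building's interactions.
; It spawns its default controller at BeginPlay so it can navigate.
; AssigntoBuilding stops interactions on any previous building, stores the new one and uses AIMoveTo to walk there.
; On arrival, it calls DoInteraction on each entry in the building's Interactions list, passing the building and itself.
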(event `self.ReceiveBeginPlay`
  (`self.SpawnDefaultController`))

(event `Assign to Building`
  (params (Building :type "/Game/TitanGamez/Buildings/BP_Building_Base Object Reference"))
  ;[1 1 1] Assign to Building
  (`|ExecutionSequence`
    (:`then_0`
      (`/Engine/EditorBlueprintResources/StandardMacros.IsValid` (`self.Building Assigned`) ; Be sure this is not the first time we assign\nbuilding - if yes, ignore stopping current\ninteractions
        (:`Is Valid`
          (`self.Stop Interactions`))))
    (:`then_1`
      (bind _output_get (set `self.Building Assigned` Building))
      (`|AIMoveTo` self (0.0 0.0 0.0) _output_get 15.0 true
        (:`OnSuccess`
          (`self.Do Interactions`))))))

(event `Do Interactions`
  ;[1 1 1] Do Interactions
  (for _array_element (`Building_Base.Interactions` (`self.Building Assigned`))
    (`Interaction_Base.DoInteraction` _array_element (`self.Building Assigned`) self)))

(event `Stop Interactions`
  ;[1 1 1] Stop Interactions
  (for _array_element (`Building_Base.Interactions` (`self.Building Assigned`))
    (`Interaction_Base.StopInteraction` _array_element (`self.Building Assigned`) self)))

(fn `UserConstructionScript`)