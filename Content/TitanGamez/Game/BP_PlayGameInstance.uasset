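; Game instance Blueprint that keeps the list of buildings currently on the map.
; AddBuilding appends a building only if it is not already listed, and DelBuilding removes one; both then invoke CallUpdateActions to signal the change.
; Resetallvalues clears the list without that update call, and GetBuildings returns the array to callers.
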(event `Add Building`
  (params (Building :type "/Game/TitanGamez/Buildings/BP_Building_Base Object Reference (by ref)"))
  ;[1 1 1] Add Building to the array - only if not exist
  (if (not (> (`KismetArrayLibrary.Array_Find` (`self.Buildings on the map`) Building) -1))
    (`KismetArrayLibrary.Array_Add` (`self.Buildings on the map`) Building)
    (`self.Update Actions`)))

(event `Del Building`
  (params (Building :type "/Game/TitanGamez/Buildings/BP_Building_Base Object Reference (by ref)"))
  ;[1 1 1] Remove Building from array - only if exist
  (`KismetArrayLibrary.Array_RemoveItem` (`self.Buildings on the map`) Building)
  (`self.Update Actions`))

(event `Reset all values`
  ;[1 1 1] Reset all values
  (`KismetArrayLibrary.Array_Clear` (`self.Buildings on the map`)))

(fn `Get Buildings`
  (returns (`Buildings on the map` :type "Array of /Game/TitanGamez/Buildings/BP_Building_Base Object Reference"))
  (return (`self.Buildings on the map`)))