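; BP_StaticPawn is a pawn that sets up the on-screen interface and mouse control when play begins.
; BeginPlay runs three custom events in sequence.
; Two create the UMG_BuildingSel action selector and UMG_Menu widgets for the first player controller and add them to the viewport.
; The last shows that controller's mouse cursor, and the pawn has no tick, overlap or construction logic.
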(event `self.ReceiveBeginPlay`
  (`self.Add Action selector to Viewport`)
  (`self.Add Menu to Viewport`)
  (`self.Initialize Mouse`))

(event `Add Action selector to Viewport`
  ;[1 1 1] Add Action selector to Viewport
  (bind _returnvalue (`|CreateWidget` "/Game/TitanGamez/UI/UMG_BuildingSel.UMG_BuildingSel_C" (`GameplayStatics.GetPlayerController` 0)))
  (`UserWidget.AddToViewport` _returnvalue 0))

(event `Add Menu to Viewport`
  ;[1 1 1] Add Menu to Viewport
  (bind _returnvalue (`|CreateWidget` "/Game/TitanGamez/UI/UMG_Menu.UMG_Menu_C" (`GameplayStatics.GetPlayerController` 0)))
  (`UserWidget.AddToViewport` _returnvalue 0))

(event `Initialize Mouse`
  ;[1 1 1] Initialize Mouse
  (set `PlayerController.bShowMouseCursor` true (`GameplayStatics.GetPlayerController` 0)))

(fn `UserConstructionScript`)