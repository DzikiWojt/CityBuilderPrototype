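; BP_Interaction_ChangeMaterialLimitedRunsToAgent is an interaction that changes the mesh material of the concerned agent, with a limit on runs per agent.
; DoInteraction first checks the interaction's max-interaction limit, then the agent's run allowance, before setting Material on slot 0.
; The allowance is a countdown stored on BP_Agent as ChangeMaterialMaxRuns, decremented by the check itself.
; Agents that are not BP_Agent always fail the check.
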(event `self.DoInteraction`
  (params (Concerned_Building :type "Building_Base Object Reference") (Concerned_Agent :type "Agent_Base Object Reference"))
  ;[1 1 1] Do Interaction
  (bind _can_interact__ (`self.Check Max Interactions`))
  (if _can_interact__
    (bind _can_run__ (`self.Check Max Runs of Agent` Concerned_Agent))
    (if _can_run__
      (`PrimitiveComponent.SetMaterial` (`Character.Mesh` Concerned_Agent) 0 (`self.Material`)))))

(fn `Check Max Runs of Agent`
  (params (Agent :type "Agent_Base Object Reference"))
  (returns (`Can Run ?` :type Boolean))
  (bind _asbp_agent (cast `/Game/TitanGamez/Agent/BP_Agent` Agent)
    (:`then`
      (if (> (`/Game/TitanGamez/Agent/BP_Agent.Change Material Max Runs` _asbp_agent) 0)
        (set `/Game/TitanGamez/Agent/BP_Agent.Change Material Max Runs` (- (`/Game/TitanGamez/Agent/BP_Agent.Change Material Max Runs` _asbp_agent) 1) _asbp_agent)
        (return true)
        (else
          (return false))))
    (:`CastFailed`
      (return false))))